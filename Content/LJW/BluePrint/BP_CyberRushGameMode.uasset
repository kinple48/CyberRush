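; BP_CyberRushGameMode is a game mode that manages the main, start and game over UI for the Cyber Rush runner.
; BeginPlay shows the main and start widgets and applies audio settings from the game instance.
; Tick polls the player's IsDead flag and, through a DoOnce, removes the main widget, then after a delay plays a voice clip and shows the game over widget.
; ResetUI re-arms that DoOnce.
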(event `self.ReceiveBeginPlay`
  (bind _returnvalue (`|CreateWidget` "/Game/LJW/UI/WBP_MainWidget.WBP_MainWidget_C"))
  (bind _output_get (set `self.MainWidget` _returnvalue))
  (`UserWidget.AddToViewport` _output_get 0)
  (bind _returnvalue_2 (`|CreateWidget` "/Game/LJW/UI/WBP_StartWidget.WBP_StartWidget_C"))
  (bind _output_get_2 (set `self.StartWidgetRef` _returnvalue_2))
  (`UserWidget.AddToViewport` _output_get_2 0)
  (bind _asbp_cyber_rush_game_instance (cast `/Game/LJW/BluePrint/BP_CyberRushGameInstance` (`GameplayStatics.GetGameInstance`)))
  (`CyberRushGameInstance.ApplyAudioSettings` _asbp_cyber_rush_game_instance (`CyberRushGameInstance.GetTheWorld` _asbp_cyber_rush_game_instance)))

(event `self.ReceiveTick`
  (params (DeltaSeconds :type "Float (single-precision)"))
  (bind _asrunner_player_base (cast `RunnerPlayerBase` (`GameplayStatics.GetPlayerPawn` 0)))
  (if (`RunnerPlayerBase.bIsDead` _asrunner_player_base)
    (`/Engine/EditorBlueprintResources/StandardMacros.DoOnce` false :!label _label
      (:`Completed`
        (`Widget.RemoveFromParent` (`self.MainWidget`))
        (`KismetSystemLibrary.Delay` 1.0)
        (`GameplayStatics.PlaySound2D` "/Game/LJW/Sound/SFX/UI/game-over-deep-male-voice-clip-352695.game-over-deep-male-voice-clip-352695" 1.0 1.0 0.0 null null)
        (bind _returnvalue (`|CreateWidget` "/Game/LJW/UI/WBP_GameOverWidget.WBP_GameOverWidget_C"))
        (`UserWidget.AddToViewport` _returnvalue 0)))))

(event `ResetUI`
  (goto _label :!via `Reset`))

(fn `UserConstructionScript`)