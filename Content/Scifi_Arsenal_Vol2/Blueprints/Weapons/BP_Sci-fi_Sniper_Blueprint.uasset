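; Sci-fi sniper rifle weapon Blueprint that handles firing feedback, ammo and cosmetic customization, with no hit or projectile logic.
; Fire decrements ammo and mirrors it to My_Game_Mode, then plays the shot animation and camera shake and spawns muzzle flash and shell actors on mesh sockets.
; An empty magazine ends firing and plays a sound.
; The construction script tints rifle and scope through dynamic materials and sets scope and bipod visibility.
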(event `self.ReceiveBeginPlay`
  ;[0 1 1] Get and Store Game Mode
  (bind _asmy_game_mode (cast `/Game/Scifi_Arsenal_Vol2/Blueprints/My_Game_Mode` (`GameplayStatics.GetGameMode`)))
  (bind _output_get (set `self.My Game mode` _asmy_game_mode))
  (set `/Game/Scifi_Arsenal_Vol2/Blueprints/My_Game_Mode.Sci-fi Rifle 02 Ammo` (`self.Ammo Amount`) _output_get))

(event `Fire`
  (bind (_returnvalue_location _returnvalue_rotation _returnvalue_scale) (`KismetMathLibrary.BreakTransform` (`self.GetTransform`)))
  (bind (_returnvalue_location_2 _returnvalue_rotation_2 _returnvalue_scale_2) (`KismetMathLibrary.BreakTransform` (`self.GetTransform`)))
  (bind _skeletalmeshcomponent (`self.SkeletalMeshComponent`))
  ;[0 1 0.6016 1 25] Fire Event System
  (set `self.IsFiring?` true)
  (if (<= (`self.Ammo Amount`) 0)
    (`self.End Fire`)
    (`self.Ammo Empty`)
    (else
      (bind _ammo_result (`self.Calcuate Ammo` (`self.Ammo Amount`) :!pinned true)) ; Calculate Ammo
      (bind _output_get (set `self.Ammo Amount` _ammo_result))
      (set `/Game/Scifi_Arsenal_Vol2/Blueprints/My_Game_Mode.Sci-fi Rifle 02 Ammo` _output_get (`self.My Game mode`) :!pinned true) ; Set Ammo Variable in Game mode
      ;;[0 0.2266 1 1 25] Spawn Muzzle Flash
      (`SkeletalMeshComponent.PlayAnimation` _skeletalmeshcomponent "/Game/Scifi_Arsenal_Vol2/Animations/Animation_Sequences/Sci-fi_Sniper/Sci-fi_Sniper_Fire_Shot_Anim.Sci-fi_Sniper_Fire_Shot_Anim" false)
      (bind _returnvalue (`|SpawnActorFromClass` (`self.MuzzleFlash Actor`) (`KismetMathLibrary.MakeTransform` _returnvalue_location_2 _returnvalue_rotation_2 (* _returnvalue_scale_2 1.75)) "AlwaysSpawn" "OverrideRootScale" null null))
      (`self.K2_AttachToComponent` _returnvalue _skeletalmeshcomponent "MuzzleFlash_Socket" "SnapToTarget" "KeepWorld" "KeepRelative" true)
      ;;[0 0.4609 1 1 25] Spawn Ammo Shell
      (bind _returnvalue_2 (`|SpawnActorFromClass` (`self.Ammo Shell Actor`) (`KismetMathLibrary.MakeTransform` _returnvalue_location _returnvalue_rotation (* _returnvalue_scale 1.8)) "AlwaysSpawn" "OverrideRootScale" null null))
      (`self.K2_AttachToComponent` _returnvalue_2 _skeletalmeshcomponent "BulletShell_Socket" "SnapToTarget" "KeepWorld" "KeepRelative" true)
      ;;[40 0 0.6312] Play Camera Shake
      (`PlayerCameraManager.StartCameraShake` :`self` (`GameplayStatics.GetPlayerCameraManager` 0) :`ShakeClass` (`self.Weapon Camera Shake`)))))

(event `End Fire`
  ;[0 1 0.6016 1 25] Fire Event System
  (set `self.IsFiring?` false)
  (`KismetSystemLibrary.K2_ClearAndInvalidateTimerHandle` (`self.Fire Timer`))
  (`PlayerController.ClientStopCameraShake` (`GameplayStatics.GetPlayerController` 0) null false :!pinned true) ; Stop All Camera Shake
)

(event `Ammo Empty`
  ;[0 1 0.6016 1 25] Fire Event System
  (`GameplayStatics.PlaySound2D` (`self.Ammo Empty Sound`) 1.0 1.0 0.0 null null :!pinned true) ; Play Ammo Empty Sound
)

(event `Show Scope Attachment`
  ;[0 1 0.6016 1 25] Fire Event System
  ;;[1 0.3281 0] Set Visible Weapon Scope Skeletal Mesh Attachment
  (`SceneComponent.ToggleVisibility` (`self.Sci-fi Sniper Scope`) false))

(fn `Calcuate Ammo`
  (params (`Ammo Value` :type Integer))
  (returns (`Ammo Result` :type Integer))
  (locals (`Temp Int` :type Integer))
  (bind _output_get (set `local.Temp Int` `Ammo Value`))
  (bind _output_get_2 (set `local.Temp Int` (- _output_get 1)))
  (if (< _output_get_2 0)
    (set `local.Temp Int` 0))
  (return (`local.Temp Int`)))

(fn `Show Bipod`
  (params (Show :type Boolean))
  (`SceneComponent.SetVisibility` (`self.Sci-fi Sniper Bipod`) Show false))

(fn `Show_Scope_01`
  (params (`Show Bool` :type Boolean))
  (`SceneComponent.SetVisibility` (`self.Sci-fi Sniper Scope`) `Show Bool` false))

(fn `UserConstructionScript`
  ;[0.3333 0.3333 0.3333] Set Color at Runtime
  (bind _returnvalue (`PrimitiveComponent.CreateDynamicMaterialInstance` (`self.SkeletalMeshComponent`) 0 null "None"))
  (`MaterialInstanceDynamic.SetScalarParameterValue` _returnvalue "Blend mode" (`self.Blend mode Value`))
  (`MaterialInstanceDynamic.SetVectorParameterValue` _returnvalue "Base Color Tint" (`self.Skin_Color`))
  (bind _returnvalue_2 (`PrimitiveComponent.CreateDynamicMaterialInstance` (`self.Sci-fi Sniper Scope`) 2 null "None"))
  (`MaterialInstanceDynamic.SetScalarParameterValue` _returnvalue_2 "Blend mode" (`self.Blend mode Value`))
  (`MaterialInstanceDynamic.SetVectorParameterValue` _returnvalue_2 "Base Color Tint" (`self.Skin_Color`))
  ;[0.09272 0.09046 0.09896] Hide and show Ironsights, Scope and Bipod
  (`self.Show_Scope_01` (`|EnumEquality` (`self.Scope Types`) "NewEnumerator0"))
  (`self.Show_Scope_01` (`|EnumEquality` (`self.Scope Types`) "NewEnumerator0") :!pinned true) ; Add your Second Scope "Show_Scope_02" Function Here
  (`self.Show Bipod` (`self.Show_Bipod`))
  (`PrimitiveComponent.SetCollisionEnabled` (`self.SkeletalMeshComponent`) "NoCollision"))