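; Sci-fi rifle weapon actor that fires automatically, tracks its ammo and mirrors the count to My_Game_Mode.
; Fire starts a looping timer; each shot plays the fire animation, spawns socket-attached flash, smoke and shell actors, and shakes the camera.
; Shots raise a muzzle-heat material parameter, which EndFire resets, while an empty magazine plays a sound.
; The construction script tints the skin materials, picks ironsight or scope with ammo widget, and disables mesh collision.
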(event `self.ReceiveBeginPlay`
  ;[0 0.1797 1 1 25] Get Muzzle Material
  (bind _returnvalue (`PrimitiveComponent.CreateDynamicMaterialInstance` (`self.SkeletalMeshComponent`) 1 null "None"))
  (set `self.Muzzle Material` _returnvalue)
  ;[0 1 1 1 25] Get and Store Game Mode
  (bind _asmy_game_mode (cast `/Game/Scifi_Arsenal_Vol2/Blueprints/My_Game_Mode` (`GameplayStatics.GetGameMode`)))
  (bind _output_get (set `self.My Game Mode` _asmy_game_mode))
  (set `/Game/Scifi_Arsenal_Vol2/Blueprints/My_Game_Mode.Sci-fi Rifle 01 Ammo` (`self.Ammo Amount`) _output_get))

(event `Fire`
  ;[0 0.7891 1 1 25] Fire Event System
  (set `self.IsFiriing?` true)
  (if (<= (`self.Ammo Amount`) 0)
    (`self.End Fire`)
    (`self.Ammo Empty`)
    (else
      (`self.Automatic Fire`)
      (bind _returnvalue (`KismetSystemLibrary.K2_SetTimerDelegate` (delegate `Automatic Fire`) (`self.Fire Rate`) true))
      (set `self.Fire Timer` _returnvalue))))

(event `Automatic Fire`
  (bind (_returnvalue_location _returnvalue_rotation _returnvalue_scale) (`KismetMathLibrary.BreakTransform` (`self.GetTransform`)))
  (bind (_returnvalue_location_2 _returnvalue_rotation_2 _returnvalue_scale_2) (`KismetMathLibrary.BreakTransform` (`self.GetTransform`)))
  (bind (_returnvalue_location_3 _returnvalue_rotation_3 _returnvalue_scale_3) (`KismetMathLibrary.BreakTransform` (`self.GetTransform`)))
  (bind _skeletalmeshcomponent (`self.SkeletalMeshComponent`))
  (bind _muzzleflash_actor (`self.MuzzleFlash Actor`))
  (bind _returnvalue (`KismetMathLibrary.MakeTransform` _returnvalue_location_3 _returnvalue_rotation_3 (* _returnvalue_scale_3 0.5)))
  ;[0 0.7891 1 1 25] Fire Event System
  (if (`self.IsFiriing?`)
    (if (<= (`self.Ammo Amount`) 0)
      (`self.End Fire`)
      (`self.Ammo Empty`)
      (else
        (bind _ammo_result (`self.Calculate Ammo` (`self.Ammo Amount`) :!pinned true)) ; Calculate Ammo
        (bind _output_get (set `self.Ammo Amount` _ammo_result))
        (set `/Game/Scifi_Arsenal_Vol2/Blueprints/My_Game_Mode.Sci-fi Rifle 01 Ammo` _output_get (`self.My Game Mode`) :!pinned true) ; Set Ammo Variable in Game mode
        ;;[0 1 0.4141 1 25] Spawn Muzzle Flash and Smoke
        (`SkeletalMeshComponent.PlayAnimation` _skeletalmeshcomponent "/Game/Scifi_Arsenal_Vol2/Animations/Animation_Sequences/Sci-fi_Rifle_01/Sci-fi_Rifle_01_Fire_Anim.Sci-fi_Rifle_01_Fire_Anim" false)
        (bind _returnvalue_2 (`|SpawnActorFromClass` _muzzleflash_actor _returnvalue "AlwaysSpawn" "OverrideRootScale" null null))
        (`self.K2_AttachToComponent` _returnvalue_2 _skeletalmeshcomponent "MuzzleFlash_Socket_01" "SnapToTarget" "KeepWorld" "KeepRelative" true)
        (bind _returnvalue_3 (`|SpawnActorFromClass` _muzzleflash_actor _returnvalue "AlwaysSpawn" "OverrideRootScale" null null))
        (`self.K2_AttachToComponent` _returnvalue_3 _skeletalmeshcomponent "MuzzleFlash_Socket_02" "SnapToTarget" "KeepWorld" "KeepRelative" true)
        ;;[0.8281 1 0 1 25] Spawn Ammo Shells
        (bind _returnvalue_4 (`|SpawnActorFromClass` (`self.AmmoShell Actor`) (`KismetMathLibrary.MakeTransform` _returnvalue_location_2 _returnvalue_rotation_2 (* _returnvalue_scale_2 2.0)) "AlwaysSpawn" "OverrideRootScale" null null))
        (`self.K2_AttachToComponent` _returnvalue_4 _skeletalmeshcomponent "BulletShell_Socket" "SnapToTarget" "KeepWorld" "KeepRelative" true)
        ;;[0 0.1562 1 1 25] Spawn Smoke
        (bind _returnvalue_5 (`|SpawnActorFromClass` (`self.MuzzleSmoke Actor`) (`KismetMathLibrary.MakeTransform` _returnvalue_location _returnvalue_rotation (* _returnvalue_scale 0.6)) "AlwaysSpawn" "OverrideRootScale" null null))
        (`self.K2_AttachToComponent` _returnvalue_5 _skeletalmeshcomponent "MuzzleFlash_Socket_01" "SnapToTarget" "KeepWorld" "KeepRelative" true)
        (`MaterialInstanceDynamic.SetScalarParameterValue` (`self.Muzzle Material`) "Muzzle Heat Effect" 4.0 :!pinned true) ; Activate Muzzle Heat Effect
        ;[40 0 0.6312] Play Camera Shake
        (`PlayerCameraManager.PlayCameraShake` :`self` (`GameplayStatics.GetPlayerCameraManager` 0) :`ShakeClass` (`self.Weapon Camera Shake`))))))

(event `End Fire`
  ;[0 0.7891 1 1 25] Fire Event System
  (set `self.IsFiriing?` false)
  (`KismetSystemLibrary.K2_ClearAndInvalidateTimerHandle` (`self.Fire Timer`))
  (`MaterialInstanceDynamic.SetScalarParameterValue` (`self.Muzzle Material`) "Muzzle Heat Effect" 0.0 :!pinned true) ; Activate Muzzle Heat Effect
  (`PlayerController.ClientStopCameraShake` (`GameplayStatics.GetPlayerController` 0) "/Game/Scifi_Arsenal_Vol2/Blueprints/Weapon_CameraShake/Automatic_Weapon_CameraShake.Automatic_Weapon_CameraShake_C" false :!pinned true) ; Stop All Camera Shake
)

(event `Ammo Empty`
  ;[0 0.7891 1 1 25] Fire Event System
  (`GameplayStatics.PlaySound2D` (`self.Ammo Empty Sound`) 1.0 1.0 0.0 null null :!pinned true) ; Play Ammo Empty Sound
)

(event `Show Scope Attachment`
  ;[0 0.7891 1 1 25] Fire Event System
  ;;[1 0.3047 0] Set Visible Weapon Scope Skeletal Mesh Attachment
  (`SceneComponent.ToggleVisibility` (`self.Sci-fi Rifle 01 IronsightScope`) false)
  (`SceneComponent.ToggleVisibility` (`self.Sci-fi Rifle 01 Ironsight`) false)
  (`SceneComponent.ToggleVisibility` (`self.Ammo UMG`) false))

(fn `Calculate Ammo`
  (params (`Ammo Value` :type Integer))
  (returns (`Ammo Result` :type Integer))
  (locals (NewLocalVar_0 :type "/Game/Scifi_Arsenal_Vol2/UMG/Sci-fi_Rifle_01_AmmoCounter_WB Object Reference") (`Temp Int` :type Integer))
  (bind _output_get (set `local.Temp Int` `Ammo Value`))
  (bind _output_get_2 (set `local.Temp Int` (- _output_get 1)))
  (if (< _output_get_2 0)
    (set `local.Temp Int` 0))
  (return (`local.Temp Int`)))

(fn `Show Ironsight`
  (params (`Show Bool` :type Boolean))
  (`SceneComponent.SetVisibility` (`self.Sci-fi Rifle 01 Ironsight`) `Show Bool` false))

(fn `Show Scope`
  (params (`Show Bool` :type Boolean))
  (`SceneComponent.SetVisibility` (`self.Sci-fi Rifle 01 IronsightScope`) `Show Bool` false)
  (`SceneComponent.SetVisibility` (`self.Ammo UMG`) `Show Bool` false))

(fn `UserConstructionScript`
  (bind _weapon_ironsight_or_scope (`self.Weapon Ironsight OR Scope`))
  (bind _skeletalmeshcomponent (`self.SkeletalMeshComponent`))
  ;[0.3333 0.3333 0.3333] Set Color at Runtime
  (bind _returnvalue (`PrimitiveComponent.CreateDynamicMaterialInstance` _skeletalmeshcomponent 4 null "None"))
  (`MaterialInstanceDynamic.SetScalarParameterValue` _returnvalue "Blend mode" (`self.Blend mode Value`))
  (`MaterialInstanceDynamic.SetVectorParameterValue` _returnvalue "Base Color Tint" (`self.Skin_Color`))
  (bind _returnvalue_2 (`PrimitiveComponent.CreateDynamicMaterialInstance` _skeletalmeshcomponent 0 null "None"))
  (`MaterialInstanceDynamic.SetScalarParameterValue` _returnvalue_2 "Blend mode" (`self.Blend mode Value`))
  (`MaterialInstanceDynamic.SetVectorParameterValue` _returnvalue_2 "Base Color Tint" (`self.Skin_Color`))
  (bind _returnvalue_3 (`PrimitiveComponent.CreateDynamicMaterialInstance` _skeletalmeshcomponent 1 null "None"))
  (`MaterialInstanceDynamic.SetScalarParameterValue` _returnvalue_3 "Blend mode" (`self.Blend mode Value`))
  (`MaterialInstanceDynamic.SetVectorParameterValue` _returnvalue_3 "Base Color Tint" (`self.Skin_Color`))
  (bind _returnvalue_4 (`PrimitiveComponent.CreateDynamicMaterialInstance` _skeletalmeshcomponent 5 null "None"))
  (`MaterialInstanceDynamic.SetScalarParameterValue` _returnvalue_4 "Blend mode" (`self.Blend mode Value`))
  (`MaterialInstanceDynamic.SetVectorParameterValue` _returnvalue_4 "Base Color Tint" (`self.Skin_Color`))
  ;[0.09272 0.09046 0.09896] Hide and show Ironsights
  (`self.Show Ironsight` (`|EnumEquality` _weapon_ironsight_or_scope "NewEnumerator0"))
  (`self.Show Scope` (`|EnumEquality` _weapon_ironsight_or_scope "NewEnumerator3"))
  (`PrimitiveComponent.SetCollisionEnabled` (`self.SkeletalMeshComponent`) "NoCollision" :!pinned true) ; Remove Collision
)