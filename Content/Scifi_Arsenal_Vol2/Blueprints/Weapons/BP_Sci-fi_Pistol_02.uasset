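; Sci-fi pistol weapon actor with configurable skin tint, ironsights, scope, and laser or torchlight attachment.
; The construction script builds tinted dynamic materials and shows the chosen attachments.
; Fire decrements ammo, plays the fire animation, spawns socket-attached muzzle flash and shell actors, and shakes the camera, or plays an empty sound when out.
; Tick line-traces from the laser locator to end the beam at the first impact.
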(event `self.ReceiveTick`
  (params (DeltaSeconds :type "Float (single-precision)"))
  ;[0 1 0.3438 1 25] Fire Event
  (`self.Emit Laser Beam`))

(event `Fire`
  (bind (_returnvalue_location _returnvalue_rotation _returnvalue_scale) (`KismetMathLibrary.BreakTransform` (`self.GetTransform`)))
  (bind (_returnvalue_location_2 _returnvalue_rotation_2 _returnvalue_scale_2) (`KismetMathLibrary.BreakTransform` (`self.GetTransform`)))
  (bind _skeletalmeshcomponent (`self.SkeletalMeshComponent`))
  ;[0 1 0.3438 1 25] Fire Event
  (set `self.IsFiring?` true)
  (if (<= (`self.Ammo Amount`) 0)
    (`self.End Fire`)
    (`self.Ammo Empty`)
    (else
      (bind _ammo_result (`self.Calculate Ammo` (`self.Ammo Amount`) :!pinned true)) ; Calculate Ammo
      (set `self.Ammo Amount` _ammo_result)
      ;;[0.2891 0 1 1 26] Spawn Muzzle Flash and Bullet eject particles
      (`SkeletalMeshComponent.PlayAnimation` _skeletalmeshcomponent "/Game/Scifi_Arsenal_Vol2/Animations/Animation_Sequences/Sci-fi_Pistol_02/Sci-fi_Pistol_02_Fire_OneShot_Anim.Sci-fi_Pistol_02_Fire_OneShot_Anim" false)
      (bind _returnvalue (`|SpawnActorFromClass` (`self.MuzzleFlash Actor`) (`KismetMathLibrary.MakeTransform` _returnvalue_location_2 _returnvalue_rotation_2 (* _returnvalue_scale_2 2.0)) "AlwaysSpawn" "OverrideRootScale" null null))
      (`self.K2_AttachToComponent` _returnvalue _skeletalmeshcomponent "MuzzleFlash_Socket" "SnapToTarget" "KeepWorld" "KeepRelative" true)
      (bind _returnvalue_2 (`|SpawnActorFromClass` (`self.AmmoShell Actor`) (`KismetMathLibrary.MakeTransform` _returnvalue_location _returnvalue_rotation (* _returnvalue_scale 1.0)) "AlwaysSpawn" "OverrideRootScale" null null))
      (`self.K2_AttachToComponent` _returnvalue_2 _skeletalmeshcomponent "BulletShell_Socket" "SnapToTarget" "KeepWorld" "KeepRelative" true)
      (`GameplayStatics.PlayWorldCameraShake` (`self.Weapon Camera Shake`) (`self.K2_GetActorLocation`) 0.0 500.0 :!pinned true) ; Play Camera Shake
    )))

(event `End Fire`
  ;[0 1 0.3438 1 25] Fire Event
  (set `self.IsFiring?` false))

(event `Ammo Empty`
  ;[0 1 0.3438 1 25] Fire Event
  (`GameplayStatics.PlaySound2D` (`self.Ammo Empty Sound`) 1.0 0.6 0.0 null null :!pinned true) ; Play Ammo Empty Sound
)

(event `Show Scope Attachment`
  ;[0 1 0.3438 1 25] Fire Event
  ;;[0.2422 0 1] Set Visible Weapon Scope Skeletal Mesh Attachment
  (`SceneComponent.ToggleVisibility` (`self.Sci-fi Pistol 02 Scope`) false)
  (`SceneComponent.ToggleVisibility` (`self.Scope Target Widget`) false))

(fn `Calculate Ammo`
  (params (`Ammo Value` :type Integer))
  (returns (`Ammo Result` :type Integer))
  (locals (`Temp Int` :type Integer))
  (bind _output_get (set `local.Temp Int` `Ammo Value`))
  (bind _output_get_2 (set `local.Temp Int` (- _output_get 1)))
  (if (< _output_get_2 0)
    (set `local.Temp Int` 0))
  (return (`local.Temp Int`)))

(fn `Emit Laser Beam`
  (bind _laser_beam_start_locator (`self.Laser Beam Start Locator`))
  (bind _returnvalue (`SceneComponent.K2_GetComponentLocation` _laser_beam_start_locator))
  (bind _returnvalue_2 (+ _returnvalue (* (`SceneComponent.GetForwardVector` _laser_beam_start_locator) (`self.Trace Distance`))))
  ;[0.3333 0.3333 0.3333] Trace and get hit Location along Laser Beam path
  (bind (_outhit _returnvalue_3) (`KismetSystemLibrary.LineTraceSingle` _returnvalue _returnvalue_2 "TraceTypeQuery1" true (`|MakeArray` self :!type "Actor Object Reference")))
  (`ParticleSystemComponent.SetBeamTargetPoint` (`self.P_LaserBeam`) 0 (`KismetMathLibrary.SelectVector` (`.Location` (`GameplayStatics.BreakHitResult` _outhit)) _returnvalue_2 _returnvalue_3) 0 :!pinned true) ; Set the laser beam to end at impact
)

(fn `Show_Ironsight_01`
  (params (`Show Bool` :type Boolean))
  (`SceneComponent.SetVisibility` (`self.Sci-fi Pistol 02 Ironsight 02`) `Show Bool` false))

(fn `Show_Ironsight_02`
  (params (`Show Bool` :type Boolean))
  (`SceneComponent.SetVisibility` (`self.Sci-fi Pistol 02 Ironsight 01`) `Show Bool` false))

(fn `Show_Laser`
  (params (`Show Bool` :type Boolean))
  (`SceneComponent.SetVisibility` (`self.Sci-fi Pistol 02 Attachment Laser`) `Show Bool` false)
  (`SceneComponent.SetVisibility` (`self.P_LaserBeam`) `Show Bool` false))

(fn `Show_Scope`
  (params (`Show Bool` :type Boolean))
  (`SceneComponent.SetVisibility` (`self.Sci-fi Pistol 02 Scope`) `Show Bool` false)
  (`SceneComponent.SetVisibility` (`self.Scope Target Widget`) `Show Bool` false))

(fn `Show_Touchlight`
  (params (`Show Bool` :type Boolean))
  (`SceneComponent.SetVisibility` (`self.Sci-fi Pistol 02 Attachment Touchlight`) `Show Bool` false)
  (`SceneComponent.SetVisibility` (`self.Touchlight`) `Show Bool` false))

(fn `UserConstructionScript`
  (bind _weaponattachmenttype (`self.WeaponAttachmentType`))
  (bind _weaponironsighttype (`self.WeaponIronsightType`))
  (bind _skeletalmeshcomponent (`self.SkeletalMeshComponent`))
  ;[0.3333 0.3333 0.3333] Set Color at Runtime
  (bind _returnvalue (`PrimitiveComponent.CreateDynamicMaterialInstance` _skeletalmeshcomponent 1 null "None"))
  (`MaterialInstanceDynamic.SetScalarParameterValue` _returnvalue "Blend Mode" (`self.Blend mode Value`))
  (`MaterialInstanceDynamic.SetVectorParameterValue` _returnvalue "Base Color Tint" (`self.Skin_Color`))
  (bind _returnvalue_2 (`PrimitiveComponent.CreateDynamicMaterialInstance` _skeletalmeshcomponent 2 null "None"))
  (`MaterialInstanceDynamic.SetScalarParameterValue` _returnvalue_2 "Blend Mode" (`self.Blend mode Value`))
  (`MaterialInstanceDynamic.SetVectorParameterValue` _returnvalue_2 "Base Color Tint" (`self.Skin_Color`))
  (bind _returnvalue_3 (`PrimitiveComponent.CreateDynamicMaterialInstance` (`self.Sci-fi Pistol 02 Attachment Touchlight`) 0 null "None"))
  (`MaterialInstanceDynamic.SetScalarParameterValue` _returnvalue_3 "Blend Mode" (`self.Blend mode Value`))
  (`MaterialInstanceDynamic.SetVectorParameterValue` _returnvalue_3 "Base Color Tint" (`self.Skin_Color`))
  (bind _returnvalue_4 (`PrimitiveComponent.CreateDynamicMaterialInstance` (`self.Sci-fi Pistol 02 Attachment Laser`) 0 null "None"))
  (`MaterialInstanceDynamic.SetScalarParameterValue` _returnvalue_4 "Blend Mode" (`self.Blend mode Value`))
  (`MaterialInstanceDynamic.SetVectorParameterValue` _returnvalue_4 "Base Color Tint" (`self.Skin_Color`))
  ;[0.09272 0.09046 0.09896] Hide and show Ironsights
  (`self.Show_Ironsight_01` (`|EnumEquality` _weaponironsighttype "NewEnumerator0"))
  (`self.Show_Ironsight_02` (`|EnumEquality` _weaponironsighttype "NewEnumerator3"))
  (`self.Show_Scope` (`self.Show Scope`))
  (`self.Show_Laser` (`|EnumEquality` _weaponattachmenttype "NewEnumerator0"))
  (`self.Show_Touchlight` (`|EnumEquality` _weaponattachmenttype "NewEnumerator3"))
  (`PrimitiveComponent.SetCollisionEnabled` (`self.SkeletalMeshComponent`) "NoCollision"))