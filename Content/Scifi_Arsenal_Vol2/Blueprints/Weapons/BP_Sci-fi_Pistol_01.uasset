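; Sci-fi pistol weapon actor that handles single-shot firing, ammo and cosmetic setup.
; Fire decrements ammo clamped at zero, plays the fire animation, spawns socket-attached muzzle flash and shell actors, and triggers a camera shake, or plays an empty sound when out.
; The construction script tints a dynamic material with the skin color, toggles two ironsight meshes by type, and disables mesh collision.
; Fire spawns no projectile or trace, and the camera shake functions are empty stubs.
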(event `Fire`
  (bind (_returnvalue_location _returnvalue_rotation _returnvalue_scale) (`KismetMathLibrary.BreakTransform` (`self.GetTransform`)))
  (bind (_returnvalue_location_2 _returnvalue_rotation_2 _returnvalue_scale_2) (`KismetMathLibrary.BreakTransform` (`self.GetTransform`)))
  (bind _skeletalmeshcomponent (`self.SkeletalMeshComponent`))
  ;[0 0.625 1 1 25] Fire Event
  (set `self.IsFiring?` true)
  (if (<= (`self.Ammo Amount`) 0)
    (`self.End Fire`)
    (`self.Ammo Empty`)
    (else
      (bind _ammo_result (`self.Calculate` (`self.Ammo Amount`) :!pinned true)) ; Calculate Ammo
      (set `self.Ammo Amount` _ammo_result)
      ;;[0.2891 0 1 1 26] Spawn Muzzle Flash and Bullet eject particles
      (`SkeletalMeshComponent.PlayAnimation` _skeletalmeshcomponent "/Game/Scifi_Arsenal_Vol2/Animations/Animation_Sequences/Sci-fi_Pistol_01/Sci-fi_Pistol_01_Fire_OneShot_Anim.Sci-fi_Pistol_01_Fire_OneShot_Anim" false)
      (bind _returnvalue (`|SpawnActorFromClass` (`self.MuzzleFlash Actor`) (`KismetMathLibrary.MakeTransform` _returnvalue_location _returnvalue_rotation (* _returnvalue_scale 0.8)) "AlwaysSpawn" "OverrideRootScale" null null))
      (`self.K2_AttachToComponent` _returnvalue _skeletalmeshcomponent "MuzzleFlash_Socket" "SnapToTarget" "KeepWorld" "KeepRelative" true)
      (bind _returnvalue_2 (`|SpawnActorFromClass` (`self.AmmoShell Actor`) (`KismetMathLibrary.MakeTransform` _returnvalue_location_2 _returnvalue_rotation_2 (* _returnvalue_scale_2 1.0)) "AlwaysSpawn" "OverrideRootScale" null null))
      (`self.K2_AttachToComponent` _returnvalue_2 _skeletalmeshcomponent "BulletShell_Socket" "SnapToTarget" "KeepWorld" "KeepRelative" true)
      (`GameplayStatics.PlayWorldCameraShake` (`self.Weapon Camera Shake`) (`self.K2_GetActorLocation`) 0.0 500.0 :!pinned true) ; Play Camera Shake
    )))

(event `End Fire`
  ;[0 0.625 1 1 25] Fire Event
  (set `self.IsFiring?` false))

(event `Ammo Empty`
  ;[0 0.625 1 1 25] Fire Event
  (`GameplayStatics.PlaySound2D` (`self.Ammo Empty Sound`) 1.0 0.4 0.0 null null :!pinned true) ; Play Ammo Empty Sound
)

(fn `Calculate`
  (params (`Ammo Value` :type Integer))
  (returns (`Ammo Result` :type Integer))
  (locals (`Temp Int` :type Integer))
  (bind _output_get (set `local.Temp Int` `Ammo Value`))
  (bind _output_get_2 (set `local.Temp Int` (- _output_get 1)))
  (if (< _output_get_2 0)
    (set `local.Temp Int` 0))
  (return (`local.Temp Int`)))

(fn `End Camera Shake`)

(fn `Perform Camera Shake`)

(fn `Show_Ironsight_01`
  (params (`Show Bool` :type Boolean))
  (`SceneComponent.SetVisibility` (`self.Sci-fi Pistol 01 Ironsight 01`) `Show Bool` false))

(fn `Show_Ironsight_02`
  (params (`Show Bool` :type Boolean))
  (`SceneComponent.SetVisibility` (`self.Sci-fi Pistol 01 Ironsight 02`) `Show Bool` false))

(fn `UserConstructionScript`
  (bind _weapon_ironsight_type (`self.Weapon Ironsight Type`))
  ;[0.3333 0.3333 0.3333] Set Color at Runtime
  (bind _returnvalue (`PrimitiveComponent.CreateDynamicMaterialInstance` (`self.SkeletalMeshComponent`) 3 null "None"))
  (`MaterialInstanceDynamic.SetScalarParameterValue` _returnvalue "Blend mode" (`self.Blend mode Value`))
  (`MaterialInstanceDynamic.SetVectorParameterValue` _returnvalue "Base Color Tint" (`self.Skin_Color`))
  ;[0.09272 0.09046 0.09896] Hide and show Ironsights
  (`self.Show_Ironsight_01` (`|EnumEquality` _weapon_ironsight_type "NewEnumerator0"))
  (`self.Show_Ironsight_02` (`|EnumEquality` _weapon_ironsight_type "NewEnumerator3"))
  (`PrimitiveComponent.SetCollisionEnabled` (`self.SkeletalMeshComponent`) "NoCollision"))