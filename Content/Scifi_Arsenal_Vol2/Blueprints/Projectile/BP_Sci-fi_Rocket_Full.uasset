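; Sci-fi rocket projectile actor that flies with its wings opening after spawn and removes itself after a set lifespan.
; The construction script sets the projectile velocity, applying speed to the X component only, and assigns the rocket sound.
; BeginPlay plays the wing-opening animation, then loops the opened pose after a short delay.
; Overlapping an actor or component tagged Walls destroys the rocket, with explosion effects left to be implemented there.
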(event `self.ReceiveBeginPlay`
  (bind _skeletalmeshcomponent (`self.SkeletalMeshComponent`))
  ;[0.03075 0.6644 1 1 22] Play open Wings Animation
  (`SkeletalMeshComponent.PlayAnimation` _skeletalmeshcomponent "/Game/Scifi_Arsenal_Vol2/Animations/Animation_Sequences/Sci-fi_Rocket/Sci-fi_Rocket_Wings_Opening_AnimSequence.Sci-fi_Rocket_Wings_Opening_AnimSequence" false)
  (`KismetSystemLibrary.Delay` 0.2)
  (`SkeletalMeshComponent.PlayAnimation` _skeletalmeshcomponent "/Game/Scifi_Arsenal_Vol2/Animations/Animation_Sequences/Sci-fi_Rocket/Sci-fi_Rocket_Wings_Opened_AnimSequence.Sci-fi_Rocket_Wings_Opened_AnimSequence" true)
  ;[0 1 0.1328 1 22] Destroy Self after some amount of time.
  (`self.SetLifeSpan` (`self.Projectile Lifespan`)))

(event `self.Collsion Detect Actor.OnComponentBeginOverlap`
  (params (OverlappedComponent :type "PrimitiveComponent Object Reference") (OtherActor :type "Actor Object Reference") (OtherComp :type "PrimitiveComponent Object Reference") (OtherBodyIndex :type Integer) (bFromSweep :type Boolean) (SweepResult :type "HitResult Structure (by ref)"))
  ;[1 0 0.4453 1 25] Here you Implement Explosion On Overlap Detection
  (if (or (`self.ActorHasTag` OtherActor "Walls") (`ActorComponent.ComponentHasTag` OtherComp "Walls"))
    (`self.K2_DestroyActor`)))

(fn `UserConstructionScript`
  ;[0.6406 0 1 1 22] Set Projectile Movement Variables
  (set `MovementComponent.Velocity` (`KismetMathLibrary.MakeVector` (* (`self.Speed`) (.x (`self.Velocity Direction`))) (.y (`self.Velocity Direction`)) (.z (`self.Velocity Direction`))) (`self.ProjectileMovement`))
  ;[1 0 0.4687] Play Sound
  (`AudioComponent.SetSound` (`self.Sound`) (`self.Rocket Sfx`)))