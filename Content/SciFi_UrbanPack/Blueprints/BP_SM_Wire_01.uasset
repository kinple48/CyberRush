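; Spline-driven wire prop from the SciFi Urban pack that builds a bendable run of wire along an editable spline.
; The construction script adds one spline mesh component per segment between consecutive spline points and attaches it to TopScene.
; Each segment takes its start and end positions and tangents from the spline in local space, so the pieces follow the curve.
; The event graph holds only disabled stub events, with no runtime logic.
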(fn `UserConstructionScript`
  (for _index (range (+ (- (`SplineComponent.GetNumberOfSplinePoints` (`self.Spline`)) 2) 1))
    (bind _returnvalue (`AddComponent|NODE_AddSplineMeshComponent-0` :`bManualAttachment` true))
    (`SceneComponent.K2_AttachTo` _returnvalue (`self.TopScene`) "None" "KeepRelativeOffset" true)
    (bind (_location _tangent) (`SplineComponent.GetLocationAndTangentAtSplinePoint` (`self.Spline`) _index "Local"))
    (bind (_location_2 _tangent_2) (`SplineComponent.GetLocationAndTangentAtSplinePoint` (`self.Spline`) (+ _index 1) "Local"))
    (`SplineMeshComponent.SetStartAndEnd` _returnvalue _location _tangent _location_2 _tangent_2 true)))